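; BP_WordGameMod is a game mod Blueprint that shows and hides the loading screen around game loading.
; NotifyonLoadedGame creates a UMG_Loading widget, stores it and adds it to the viewport.
; NotifyLoadedGame waits briefly, then removes that widget if it is still valid.
; GetWidgetObject returns MWidget cast to UMG_WorldView, while BeginPlay and Tick are empty.
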(event `self.ReceiveBeginPlay`)

(event `self.NotifyOnLoadedGame`
  (bind _returnvalue (`|CreateWidget` "/Game/Game/UI/UMG_Loading.UMG_Loading_C"))
  (bind _output_get (set `self.loadingWidget` _returnvalue))
  (`UserWidget.AddToViewport` _output_get 0))

(event `self.NotifyLoadedGame`
  (bind _loadingwidget (`self.loadingWidget`))
  (`KismetSystemLibrary.Delay` 1.0)
  (`/Engine/EditorBlueprintResources/StandardMacros.IsValid` _loadingwidget
    (:`Is Valid`
      (`Widget.RemoveFromParent` _loadingwidget))))

(fn `GetWidgetObject`
  (returns (`AsUMG World View` :type "/Game/Game/UI/WorldMapUmgs/UMG_WorldView Object Reference"))
  (bind _asumg_world_view (cast `/Game/Game/UI/WorldMapUmgs/UMG_WorldView` (`self.m_widget`)))
  (return _asumg_world_view))

(fn `UserConstructionScript`)