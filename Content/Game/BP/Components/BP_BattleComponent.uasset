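; Battle component that drives the on-screen indicator for the owner's attack direction.
; It creates a UMG_DirectionOfBattleWidget on BeginPlay and adds it to the viewport.
; On each battle direction change, it shows the widget and passes it the attack direction, or hides it when the HUD flag is off.
; The direction handler is marked as temporary Blueprint logic, and the Tick and empty-handed events are empty.
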(event `self.ReceiveBeginPlay`
  (bind _returnvalue (`|CreateWidget` "/Game/Game/UI/Hud/UMG_DirectionOfBattleWidget.UMG_DirectionOfBattleWidget_C"))
  (bind _output_get (set `self.BattleDirectionUi` _returnvalue))
  (`Widget.SetVisibility` _output_get "Visible")
  (`UserWidget.AddToViewport` _output_get 0))

(event `self.OnBattleDirectionChange`
  (bind _battledirectionui (`self.BattleDirectionUi`))
  ;[1 1 1] 临时用蓝图
  (if (`self.m_needShowDirectionHud`)
    (`Widget.SetVisibility` _battledirectionui "Visible")
    (`/Game/Game/UI/Hud/UMG_DirectionOfBattleWidget.On Battle Direction Change` (`self.BattleDirectionUi`) (`self.m_attackDirection`))
    (else
      (`Widget.SetVisibility` _battledirectionui "Hidden"))))

(event `self.onEmptyHanded`)